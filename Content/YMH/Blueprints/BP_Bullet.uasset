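; BP_Bullet is a simple projectile actor that flies straight ahead and removes itself after a short lifetime.
; Each Tick moves the actor with a swept SetActorLocation along the Bullet component's forward vector, using Dest as speed scaled by delta time.
; A Destroy counter increments every frame and destroys the actor past a fixed threshold, so lifetime depends on frame rate.
; The graphs contain no hit or damage handling.
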(event EventTick
  (params (DeltaSeconds :type Float%20%28single-precision%29))
  (bind _bullet (Variables|Default|GetBullet))
  (bind _result (Math|Float|IncrementFloat (Variables|Default|Getdestroy))
    (:%20%20
      (bind _output_get (Variables|Default|Setdestroy _result))
      (Transformation|SetActorLocation (+ (Transformation|GetWorldLocation _bullet) (* (Math|Vector|GetForwardVector _bullet) (Variables|Default|GetDest) DeltaSeconds)) true false)
      (if (> _output_get 1e+02)
        (Actor|DestroyActor)))))

(fn ConstructionScript)